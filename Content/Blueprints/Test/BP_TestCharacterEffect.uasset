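; BP_TestCharacterEffect is a test Blueprint that plays a camera shake in response to an OnCameraShake event.
; On BeginPlay it runs the parent logic, then binds its handler to OnCameraShake.
; The handler prints a debug message and starts CameraShakeClass on player 0's camera manager.
; Tick and overlap events are disabled placeholders, and the construction script only calls the parent.
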(event `self.ReceiveBeginPlay`
  (`parent.ReceiveBeginPlay`)
  (add `self.OnCameraShake` (delegate `OnCameraShake_Event`)))

(event `OnCameraShake_Event`
  (`KismetSystemLibrary.PrintString` "Hello Effect")
  (`PlayerCameraManager.StartCameraShake` :`self` (`PlayerController.PlayerCameraManager` (`GameplayStatics.GetPlayerController` 0)) :`ShakeClass` (`self.CameraShakeClass`)))

(fn `UserConstructionScript`
  (`parent.UserConstructionScript`))