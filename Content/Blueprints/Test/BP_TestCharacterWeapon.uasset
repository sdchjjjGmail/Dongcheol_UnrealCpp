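; BP_TestCharacterWeapon is a test character that equips an axe already present in the level when play begins.
; BeginPlay finds a BP_WeaponAxe actor, snaps it to the right-hand mesh socket, notifies it of pickup and stores it as CurrentWeapon.
; If the weapon casts to ConsumableWeapon, the character binds to its use-ended event, which only prints a debug message.
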(event `self.ReceiveBeginPlay`
  (`parent.ReceiveBeginPlay`)
  (bind _returnvalue (`GameplayStatics.GetActorOfClass` "/Game/Blueprints/Weapon/BP_WeaponAxe.BP_WeaponAxe_C"))
  (`/Engine/EditorBlueprintResources/StandardMacros.IsValid` _returnvalue
    (:`Is Valid`
      (`self.K2_AttachToComponent` _returnvalue (`self.Mesh`) "hand_rSocket" "SnapToTarget" "SnapToTarget" "SnapToTarget" true)
      (`WeaponActor.OnWeaponPickedup` _returnvalue self)
      (bind _output_get (set `self.CurrentWeapon` _returnvalue))
      (bind _asconsumable_weapon (cast `ConsumableWeapon` _output_get))
      (add `ConsumableWeapon.OnWeaponUseEnded` _asconsumable_weapon (delegate `OnWeaponUseEnded_이벤트`)))))

(event `OnWeaponUseEnded_이벤트`
  (`KismetSystemLibrary.PrintString` "Weapon ended"))

(fn `UserConstructionScript`
  (`parent.UserConstructionScript`))